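; AR_IngGame runs image-tracking AR: it starts a session with AR_Img_SessionConfig on BeginPlay and disables the screensaver.
; Each Tick it polls all tracked images and spawns one AR_Master per newly detected image, passing it that image through SetActor.
; The DetectImage map links images to their actors, whose transforms follow the tracked geometry every frame, with a debug outline drawn on each image.
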(event `self.ReceiveBeginPlay`
  (`ARBlueprintLibrary.StartARSession` "/Game/My_Stuff/Material/AR_Img_SessionConfig.AR_Img_SessionConfig")
  (`KismetSystemLibrary.ControlScreensaver` false))

(event `self.ReceiveTick`
  (params (DeltaSeconds :type "Float (single-precision)"))
  (bind _detectimage (`self.DetectImage`))
  (bind _returnvalue (`ARBlueprintLibrary.GetAllGeometriesByClass` "/Script/AugmentedReality.ARTrackedImage"))
  (for _array_element _returnvalue
    (bind _returnvalue_2 (`ARTrackedImage.GetDetectedImage` _array_element))
    (if (not (`BlueprintMapLibrary.Map_Contains` _detectimage _returnvalue_2))
      (bind _returnvalue_3 (`ARTrackedGeometry.GetLocalToTrackingTransform` _array_element))
      (bind _returnvalue_4 (`|SpawnActorFromClass` "/Game/My_Stuff/Blueprints/AR_Master.AR_Master_C" _returnvalue_3 "Undefined" "OverrideRootScale" null null))
      (bind _output_get (set `self.AR_Master` _returnvalue_4))
      (`BlueprintMapLibrary.Map_Add` _detectimage _returnvalue_2 _output_get)
      (`/Game/My_Stuff/Blueprints/AR_Master.Set_Actor` _output_get _returnvalue_2))
    (bind (_value _returnvalue_5) (`BlueprintMapLibrary.Map_Find` _detectimage _returnvalue_2))
    (`self.K2_SetActorTransform` _value _returnvalue_3 _returnvalue_5 false)
    (`ARBlueprintLibrary.DebugDrawTrackedGeometry` _array_element (struct :`G` 0.146726 :`B` 1.0) 0.5)))

(fn `UserConstructionScript`)